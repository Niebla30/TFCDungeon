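; BP_RuneButton is an interactable rune button that lights up green when overlapped and temporarily raises a linked Screw.
; BeginPlay applies a dynamic material instance to the rune tile mesh so its texture parameter can be swapped at runtime.
; Any overlap on the Button component swaps in the green rune texture, then chained delays trigger the Screw's up animation and later restore the texture and animate it down.
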(event OnComponentBeginOverlap(Button)
  (params (OverlappedComponent :type Primitive%20Component%20Object%20Reference) (OtherActor :type Actor%20Object%20Reference) (OtherComp :type Primitive%20Component%20Object%20Reference) (OtherBodyIndex :type Integer) (bFromSweep :type Boolean) (SweepResult :type Hit%20Result%20Structure%20%28by%20ref%29))
  (Rendering|Material|SetTextureParameterValue (Variables|Default|GetDynMat) "TexParam" "/Game/Assets/Textures/DungeonPackGreenRune_Texture.DungeonPackGreenRune_Texture")
  (Utilities|FlowControl|Delay 2.0)
  (Default|AnimateUp (Variables|Default|GetScrew))
  (Utilities|FlowControl|Delay 5.0)
  (Rendering|Material|SetTextureParameterValue (Variables|Default|GetDynMat) "TexParam" "/Game/Assets/Textures/DungeonPack_Texture.DungeonPack_Texture")
  (Default|AnimateDown (Variables|Default|GetScrew)))

(event EventBeginPlay
  (bind _returnvalue (Rendering|Material|CreateDynamicMaterialInstance "/Game/Assets/Materials/DungeonPack_MasterMat.DungeonPack_MasterMat" :!class /Script/Engine.KismetMaterialLibrary))
  (bind _output_get (Variables|Default|SetDynMat _returnvalue))
  (Rendering|Material|SetTextureParameterValue _output_get "TexParam" "/Game/Assets/Textures/DungeonPack_Texture.DungeonPack_Texture")
  (Rendering|Material|SetMaterial (Variables|Default|GetSM_Env_Tiles_Rune_04) 0 _output_get))

(event Collision|EventActorBeginOverlap
  (params (OtherActor :type Actor%20Object%20Reference)))

(event EventTick
  (params (DeltaSeconds :type Float%20%28single-precision%29)))

(fn ConstructionScript)