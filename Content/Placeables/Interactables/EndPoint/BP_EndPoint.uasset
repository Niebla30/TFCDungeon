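; BP_EndPoint is a placeable end point tied to one character, showing an aura while that owner stands inside it.
; Sphere overlap events ask EndPointBehaviour whether the owner entered or left and toggle the Aura's visibility from its answer.
; The construction script passes the Character to that component and creates dynamic materials, tinting aura and base red for CharFireBoy, blue otherwise.
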(event OnComponentEndOverlap(Sphere)
  (params (OverlappedComponent :type Primitive%20Component%20Object%20Reference) (OtherActor :type Actor%20Object%20Reference) (OtherComp :type Primitive%20Component%20Object%20Reference) (OtherBodyIndex :type Integer))
  ;[1 1 1] Controls who enter and/or leave end point
  ;;[1 1 1] If owner leaves end point, we set aura visibility to false
  (bind _returnvalue (Class|EndPointBehaviour|OnLeaveEndPoint (Variables|Default|GetEndPointBehaviour) OtherActor))
  (if _returnvalue
    (Rendering|SetVisibility (Variables|Default|GetAura) false false)))

(event OnComponentBeginOverlap(Sphere)
  (params (OverlappedComponent :type Primitive%20Component%20Object%20Reference) (OtherActor :type Actor%20Object%20Reference) (OtherComp :type Primitive%20Component%20Object%20Reference) (OtherBodyIndex :type Integer) (bFromSweep :type Boolean) (SweepResult :type Hit%20Result%20Structure%20%28by%20ref%29))
  ;[1 1 1] Controls who enter and/or leave end point
  ;;[0.4106 0.572 1] Is owner enters end point, we'll see aura
  (bind _returnvalue (Class|EndPointBehaviour|OnEnterEndPoint (Variables|Default|GetEndPointBehaviour) OtherActor))
  (Rendering|SetVisibility (Variables|Default|GetAura) _returnvalue false))

(fn ConstructionScript
  (Variables|/Script/TFCDungeon.EndPointBehaviour|SetOwnerCharacter (Variables|Default|GetEndPointBehaviour) (Variables|GamePlay|GetCharacter))
  (bind _returnvalue (Rendering|Material|CreateDynamicMaterialInstance "/Game/Assets/Materials/Aura_MasterMat.Aura_MasterMat" :!class /Script/Engine.KismetMaterialLibrary))
  (Rendering|Material|SetMaterial (Variables|Default|GetAura) 0 _returnvalue)
  (Variables|Default|SetInstMatAura _returnvalue)
  (bind _returnvalue_2 (Rendering|Material|CreateDynamicMaterialInstance "/Game/Assets/Materials/DungeonPack_MasterMat.DungeonPack_MasterMat" :!class /Script/Engine.KismetMaterialLibrary))
  (Rendering|Material|SetMaterial (Variables|Default|GetEndPointMesh) 0 _returnvalue_2)
  (Variables|Default|SetInstMatBase _returnvalue_2)
  (if (Utilities|Enum|Equal(Enum) (Variables|GamePlay|GetCharacter) "Char_FireBoy")
    (LocalVariables|SetAuraColor "(R=0.537255,G=0.078431,B=0.000000,A=1.000000)")
    (Rendering|Material|SetTextureParameterValue (Variables|Default|GetInstMatBase) "TexParam" "/Game/Assets/Textures/DungeonPack_Texture.DungeonPack_Texture")
    (else
      (LocalVariables|SetAuraColor "(R=0.000000,G=0.243137,B=0.537255,A=1.000000)")
      (Rendering|Material|SetTextureParameterValue (Variables|Default|GetInstMatBase) "TexParam" "/Game/Assets/Textures/DungeonPackBlue_Texture.DungeonPackBlue_Texture")))
  (Rendering|Material|SetVectorParameterValue (Variables|Default|GetInstMatAura) "Color" (LocalVariables|GetAuraColor) :!class /Script/Engine.MaterialInstanceDynamic))