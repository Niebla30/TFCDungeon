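; Placeable level-select frame that shows a level's name, picture, blocked state, earned diamonds and time.
; The construction script applies the level texture through a dynamic material for editor preview, and BeginPlay fills the display from the game instance's LevelsInfo by LevelId.
; Overlap by the hosting character, checked on authority against the owning character type, opens WBP_LevelSelection with mouse input unless blocked; leaving hides it and restores game input.
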(event OnComponentBeginOverlap(Collider)
  (params (OverlappedComponent :type Primitive%20Component%20Object%20Reference) (OtherActor :type Actor%20Object%20Reference) (OtherComp :type Primitive%20Component%20Object%20Reference) (OtherBodyIndex :type Integer) (bFromSweep :type Boolean) (SweepResult :type Hit%20Result%20Structure%20%28by%20ref%29))
  (bind _ishostingchar (CallFunction|IsHostingCharacter OtherActor))
  (if _ishostingchar
    (if (not (or (Variables|Default|GetIsShowingMenu) (Variables|Default|GetBlocked)))
      (bind _returnvalue (UserInterface|CreateWidget "/Game/Widgets/WBP_LevelSelection.WBP_LevelSelection_C" (Game|GetPlayerController 0)))
      (Variables|/Game/Widgets/WBP_LevelSelection.WBP_LevelSelection_C|SetLevel _returnvalue (Variables|Default|GetLevel%20Text))
      (Variables|/Game/Widgets/WBP_LevelSelection.WBP_LevelSelection_C|SetLevelId _returnvalue (Variables|Default|GetLevelId))
      (UserInterface|Viewport|AddtoViewport _returnvalue 0)
      (Input|SetInputModeGameandUI (Game|GetPlayerController 0) 0 "DoNotLock" true)
      (Variables|/Script/Engine.PlayerController|SetbShowMouseCursor (Game|GetPlayerController 0) true)
      (Variables|Default|SetIsShowingMenu true))))

(event OnComponentEndOverlap(Collider)
  (params (OverlappedComponent :type Primitive%20Component%20Object%20Reference) (OtherActor :type Actor%20Object%20Reference) (OtherComp :type Primitive%20Component%20Object%20Reference) (OtherBodyIndex :type Integer))
  (bind _ishostingchar (CallFunction|IsHostingCharacter OtherActor))
  (if (and _ishostingchar (Variables|Default|GetIsShowingMenu))
    (Default|HideMenu (stale OnComponentBeginOverlap(Collider) _returnvalue))
    (Input|SetInputModeGameOnly (Game|GetPlayerController 0))
    (Variables|/Script/Engine.PlayerController|SetbShowMouseCursor (Game|GetPlayerController 0) false)
    (Variables|Default|SetIsShowingMenu false)))

(event EventBeginPlay
  (bind _asbp_game_instance (Utilities|Casting|CastToBP_GameInstance (Game|GetGameInstance)))
  (Variables|Default|SetLevel%20Text (Class|KismetTextLibrary|TexttoUpper (.shortname (Utilities|Array|Get(acopy) (Variables|/Script/TFCDungeon.TFCDungeonGameInstance|GetLevelsInfo _asbp_game_instance) (Variables|Default|GetLevelId)))))
  (Variables|Default|SetBlocked (.blocked (Utilities|Array|Get(acopy) (Variables|/Script/TFCDungeon.TFCDungeonGameInstance|GetLevelsInfo _asbp_game_instance) (Variables|Default|GetLevelId))))
  (Rendering|Components|TextRender|SetText (Variables|Default|GetTR_LevelName) (Class|KismetTextLibrary|TexttoUpper (Variables|Default|GetLevel%20Text)))
  (Rendering|SetVisibility (Variables|Default|GetTR_Bloqued) (Variables|Default|GetBlocked) false)
  (Rendering|SetVisibility (Variables|Default|GetDiamond1) (>= (.diamonds (Utilities|Array|Get(acopy) (Variables|/Script/TFCDungeon.TFCDungeonGameInstance|GetLevelsInfo _asbp_game_instance) (Variables|Default|GetLevelId))) 1) false)
  (Rendering|SetVisibility (Variables|Default|GetDiamond2) (>= (.diamonds (Utilities|Array|Get(acopy) (Variables|/Script/TFCDungeon.TFCDungeonGameInstance|GetLevelsInfo _asbp_game_instance) (Variables|Default|GetLevelId))) 2) false)
  (Rendering|SetVisibility (Variables|Default|GetDiamond3) (>= (.diamonds (Utilities|Array|Get(acopy) (Variables|/Script/TFCDungeon.TFCDungeonGameInstance|GetLevelsInfo _asbp_game_instance) (Variables|Default|GetLevelId))) 3) false)
  (if (>= (.seconds (Utilities|Array|Get(acopy) (Variables|/Script/TFCDungeon.TFCDungeonGameInstance|GetLevelsInfo _asbp_game_instance) (Variables|Default|GetLevelId))) 1)
    (Rendering|Components|TextRender|SetText (Variables|Default|GetTR_Seconds) (Utilities|Text|ToText(Integer) (.seconds (Utilities|Array|Get(acopy) (Variables|/Script/TFCDungeon.TFCDungeonGameInstance|GetLevelsInfo _asbp_game_instance) (Variables|Default|GetLevelId)))))))

(fn ConstructionScript
  (Rendering|Components|TextRender|SetText (Variables|Default|GetTR_LevelName) (Class|KismetTextLibrary|TexttoUpper (Variables|Default|GetLevel%20Text)))
  (bind _returnvalue (Rendering|Material|CreateDynamicMaterialInstance (Variables|Default|GetFrame) 0 "/Game/Placeables/Interactables/LevelFrame/M_BackGround_Master.M_BackGround_Master" :!class /Script/Engine.PrimitiveComponent))
  (Rendering|Material|SetMaterial (Variables|Default|GetFrame) 0 _returnvalue)
  (Rendering|Material|SetTextureParameterValue _returnvalue "LevelTexture" (Variables|Default|GetLevelTexture))
  (Rendering|SetVisibility (Variables|Default|GetTR_Bloqued) (Variables|Default|GetBlocked) false))

(fn IsHostingCharacter
  (params (Actor :type Actor%20Object%20Reference))
  (Networking|SwitchHasAuthority
    (:Authority
      (bind _astfcdungeon_character (Utilities|Casting|CastToTFCDungeonCharacter Actor)
        (:then
          (bind _astfcdungeon_game_instance (Utilities|Casting|CastToTFCDungeonGameInstance (Game|GetGameInstance)))
          (bind _returnvalue (Class|TFCDungeonGameInstance|GetOwningCharacter _astfcdungeon_game_instance))
          (return (Utilities|Enum|Equal(Enum) _returnvalue (Variables|/Script/TFCDungeon.TFCDungeonCharacter|GetCharType _astfcdungeon_character))))
        (:CastFailed
          _)))
    (:Remote
      _))
  (return false))