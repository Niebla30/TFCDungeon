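; BP_SlidingPlatform is a placeable platform that slides between its starting location and an offset from it.
; The location is cached at BeginPlay, then the VectorSigmoid timeline scales Offset by its curve and teleports the actor without sweeping.
; AnimateForward and AnimateBackward both call Play at Speed, and AnimatePause stops playback.
; OnPostAnimate runs when the timeline finishes.
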(event EventBeginPlay
  (Variables|Default|SetInitialPosition (Transformation|GetActorLocation)))

(event EventAnimatePause
  (if (Audio|Components|Audio|IsPlaying (Variables|Default|GetVectorSigmoid))
    (bind _curvevalue (Timeline|VectorSigmoid Stop)
      (:Update
        (Transformation|SetActorLocation (+ (* _curvevalue (Variables|Default|GetOffset)) (Variables|Default|GetInitialPosition)) false true))
      (:Finished
        (Class|ActivableActor|OnPostAnimate)))))

(event EventAnimateForward
  (Components|Timeline|SetPlayRate (Variables|Default|GetVectorSigmoid) (Variables|Default|GetSpeed))
  (bind _curvevalue (Timeline|VectorSigmoid Play)
    (:Update
      (Transformation|SetActorLocation (+ (* _curvevalue (Variables|Default|GetOffset)) (Variables|Default|GetInitialPosition)) false true))
    (:Finished
      (Class|ActivableActor|OnPostAnimate))))

(event EventAnimateBackward
  (Components|Timeline|SetPlayRate (Variables|Default|GetVectorSigmoid) (Variables|Default|GetSpeed))
  (bind _curvevalue (Timeline|VectorSigmoid Play)
    (:Update
      (Transformation|SetActorLocation (+ (* _curvevalue (Variables|Default|GetOffset)) (Variables|Default|GetInitialPosition)) false true))
    (:Finished
      (Class|ActivableActor|OnPostAnimate))))

(fn ConstructionScript)