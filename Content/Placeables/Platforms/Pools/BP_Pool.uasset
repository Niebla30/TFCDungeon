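; BP_Pool is an elemental hazard pool that kills any dungeon character whose element differs from its own.
; The construction script sets the surface texture and post-process tint from the pool's element.
; A fatal overlap flags the player as dying, switches to UI-only input and plays a timeline-driven dissolve material in element colors.
; When the timeline finishes, it destroys the character, removes the HUD and calls PlayerDeath on the game state.
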(event Custom|Dissolve
  (params (Character :type TFC%20Dungeon%20Character%20Object%20Reference))
  (bind _returnvalue (Game|GetGameState))
  (Variables|Default|SetSKMesh (Variables|/Script/Engine.Character|GetMesh Character))
  (bind _returnvalue_2 (Rendering|Material|CreateDynamicMaterialInstance "/Game/MaterialLibrary/MI_Dissolve.MI_Dissolve" :!class /Script/Engine.KismetMaterialLibrary))
  (bind _output_get (Variables|Default|SetDisolveMaterial _returnvalue_2))
  (Rendering|Material|SetVectorParameterValue _output_get "Base Color" (.Value (Utilities|Map|Find (Variables|Default|GetBaseDissolveColor) (Variables|GamePlay|GetElement))) :!class /Script/Engine.MaterialInstanceDynamic)
  (Rendering|Material|SetVectorParameterValue _output_get "Fringe Color" (.Value (Utilities|Map|Find (Variables|Default|GetFringeDissolveColor) (Variables|GamePlay|GetElement))) :!class /Script/Engine.MaterialInstanceDynamic)
  (for (_ _array_index) (Rendering|Material|GetMaterials (Variables|Default|GetSKMesh))
    (Rendering|Material|SetMaterial (Variables|Default|GetSKMesh) _array_index (Variables|Default|GetDisolveMaterial)))
  (Components|Timeline|SetPlayRate (Variables|Default|GetTL_Disolve) 1.0)
  (bind _disolveamount (Timeline|TL_Disolve PlayFromStart)
    (:Update
      (Rendering|Material|SetScalarParameterValue (Variables|Default|GetDisolveMaterial) "Dissolve Amount" _disolveamount :!class /Script/Engine.MaterialInstanceDynamic))
    (:Finished
      (Actor|DestroyActor Character)
      (bind _asbp_game_state (Utilities|Casting|CastToBP_GameState _returnvalue))
      (Widget|RemovefromParent (Variables|/Game/Core/BP_GameState.BP_GameState_C|GetHudUserWidget _asbp_game_state))
      (bind _astfcdungeon_game_state (Utilities|Casting|CastToTFCDungeonGameState _returnvalue))
      (Class|TFCDungeonGameState|PlayerDeath _astfcdungeon_game_state))))

(event Collision|EventActorBeginOverlap
  (params (OtherActor :type Actor%20Object%20Reference))
  (bind _astfcdungeon_character (Utilities|Casting|CastToTFCDungeonCharacter OtherActor))
  (if (Utilities|Enum|NotEqual(Enum) (Variables|/Script/TFCDungeon.TFCDungeonCharacter|GetElement _astfcdungeon_character) (Variables|GamePlay|GetElement))
    (Variables|/Script/TFCDungeon.TFCDungeonCharacter|SetPlayerDying _astfcdungeon_character true)
    (bind _astfcdungeon_game_state (Utilities|Casting|CastToTFCDungeonGameState (Game|GetGameState)))
    (Variables|/Script/TFCDungeon.TFCDungeonGameState|SetPlayerDying _astfcdungeon_game_state true)
    (Input|SetInputModeUIOnly (Game|GetPlayerController 0) 0 "DoNotLock")
    (CallFunction|Dissolve _astfcdungeon_character)))

(fn ConstructionScript
  (bind _returnvalue (Rendering|Material|CreateDynamicMaterialInstance "/Game/Placeables/Platforms/Pools/M_Pool.M_Pool" :!class /Script/Engine.KismetMaterialLibrary))
  (Rendering|Material|SetMaterial (Variables|Default|GetSurface) 0 _returnvalue)
  (Variables|Default|SetSurfaceMatInst _returnvalue)
  (switch Utilities|FlowControl|Switch|SwitchonEElement (Variables|GamePlay|GetElement)
    (:Plasm
      (Rendering|Material|SetTextureParameterValue (Variables|Default|GetSurfaceMatInst) "TexParam" "/Game/Placeables/Platforms/Pools/T_Pool_Lava.T_Pool_Lava")
      (Variables|/Script/Engine.PostProcessComponent|SetSettings (Variables|Default|GetPostProcess) (Utilities|Struct|MakePostProcessSettings "(R=0.179050,G=0.000000,B=0.317708,A=1.000000)" "DOFM_Gaussian")))
    (:Fire
      (Rendering|Material|SetTextureParameterValue (Variables|Default|GetSurfaceMatInst) "TexParam" "/Game/Placeables/Platforms/Pools/T_Pool_Lava.T_Pool_Lava")
      (Variables|/Script/Engine.PostProcessComponent|SetSettings (Variables|Default|GetPostProcess) (Utilities|Struct|MakePostProcessSettings "(R=1.000000,G=0.073312,B=0.000000,A=1.000000)" "DOFM_Gaussian")))
    (:Water
      (Rendering|Material|SetTextureParameterValue (Variables|Default|GetSurfaceMatInst) "TexParam" "/Game/Placeables/Platforms/Pools/T_Pool_Water.T_Pool_Water")
      (Variables|/Script/Engine.PostProcessComponent|SetSettings (Variables|Default|GetPostProcess) (Utilities|Struct|MakePostProcessSettings "(R=0.000000,G=0.327850,B=0.395833,A=1.000000)" "DOFM_Gaussian")))
    (:Poison
      (Rendering|Material|SetTextureParameterValue (Variables|Default|GetSurfaceMatInst) "TexParam" "/Game/Placeables/Platforms/Pools/T_Pool_Poison.T_Pool_Poison")
      (Variables|/Script/Engine.PostProcessComponent|SetSettings (Variables|Default|GetPostProcess) (Utilities|Struct|MakePostProcessSettings "(R=0.009467,G=0.203125,B=0.021937,A=1.000000)" "DOFM_Gaussian")))))