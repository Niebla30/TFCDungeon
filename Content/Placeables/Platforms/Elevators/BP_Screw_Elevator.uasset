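; Screw elevator placeable that raises and lowers itself while its screw mesh spins.
; Timeline_0 drives both the root's height offset from the location stored at BeginPlay and the screw's yaw.
; Animate_Up and Animate_Down share one FlipFlop that alternates playing and reversing the timeline, so either event simply toggles direction.
; An InAnimation flag ignores new triggers until the timeline finishes.
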(event Custom|Animate_Up
  (bind _initiallocation (Variables|Default|GetInitialLocation))
  (if (not (Variables|Default|GetbInAnimation))
    (Variables|Default|SetbInAnimation true)
    (Utilities|FlowControl|FlipFlop
      (:A
        (bind (_direction _elevation _angle) (Timeline|Timeline_0 Play)
          (:Update
            (Transformation|SetWorldLocation (Variables|Default|GetDefaultSceneRoot) (Math|Vector|MakeVector (.x _initiallocation) (.y _initiallocation) (+ _elevation (.z _initiallocation))) false false)
            (Transformation|SetRelativeRotation (Variables|Default|Getscrew) (Math|Rotator|MakeRotator 0.0 0.0 _angle) false false))
          (:Finished
            (Variables|Default|SetbInAnimation false))))
      (:B
        (Timeline|Timeline_0 Reverse)))))

(event Custom|Animate_Down
  (bind _initiallocation (Variables|Default|GetInitialLocation))
  (if (not (Variables|Default|GetbInAnimation))
    (Variables|Default|SetbInAnimation true)
    (Utilities|FlowControl|FlipFlop
      (:A
        (bind (_direction _elevation _angle) (Timeline|Timeline_0 Play)
          (:Update
            (Transformation|SetWorldLocation (Variables|Default|GetDefaultSceneRoot) (Math|Vector|MakeVector (.x _initiallocation) (.y _initiallocation) (+ _elevation (.z _initiallocation))) false false)
            (Transformation|SetRelativeRotation (Variables|Default|Getscrew) (Math|Rotator|MakeRotator 0.0 0.0 _angle) false false))
          (:Finished
            (Variables|Default|SetbInAnimation false))))
      (:B
        (Timeline|Timeline_0 Reverse)))))

(event EventBeginPlay
  (Variables|Default|SetInitialLocation (Transformation|GetWorldLocation (Variables|Default|GetDefaultSceneRoot))))

(fn ConstructionScript)