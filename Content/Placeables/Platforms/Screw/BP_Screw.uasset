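; BP_Screw is a placeable screw in the platforms set that moves vertically while spinning.
; BeginPlay caches the root's world location as the baseline for the motion.
; The Animate_Up and Animate_Down events each drive their own timeline, one played from start and the other reversed from end.
; Each timeline update offsets the root's Z by an Elevation track and sets the Screw's relative yaw from an Angle track.
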(event Custom|Animate_Up
  (bind _initiallocation (Variables|Default|GetInitialLocation))
  (bind (_direction _elevation _angle) (Timeline|Timeline_0 PlayFromStart)
    (:Update
      (Transformation|SetWorldLocation (Variables|Default|GetDefaultSceneRoot) (Math|Vector|MakeVector (.x _initiallocation) (.y _initiallocation) (+ _elevation (.z _initiallocation))) false false)
      (Transformation|SetRelativeRotation (Variables|Default|Getscrew) (Math|Rotator|MakeRotator 0.0 0.0 _angle) false false))))

(event Custom|Animate_Down
  (bind _initiallocation (Variables|Default|GetInitialLocation))
  (bind (_direction _elevation _angle) (Timeline|Timeline_1 ReverseFromEnd)
    (:Update
      (Transformation|SetWorldLocation (Variables|Default|GetDefaultSceneRoot) (Math|Vector|MakeVector (.x _initiallocation) (.y _initiallocation) (+ _elevation (.z _initiallocation))) false false)
      (Transformation|SetRelativeRotation (Variables|Default|Getscrew) (Math|Rotator|MakeRotator 0.0 0.0 _angle) false false))))

(event EventBeginPlay
  (Variables|Default|SetInitialLocation (Transformation|GetWorldLocation (Variables|Default|GetDefaultSceneRoot))))

(event Collision|EventActorBeginOverlap
  (params (OtherActor :type Actor%20Object%20Reference)))

(event EventTick
  (params (DeltaSeconds :type Float%20%28single-precision%29)))

(fn ConstructionScript)