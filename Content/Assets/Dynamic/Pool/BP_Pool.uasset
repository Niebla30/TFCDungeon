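; BP_Pool is a pool actor whose Element setting makes it appear as lava, water or poison.
; The construction script puts a dynamic instance of ToonWater_Master on Surface and sets its toon texture for the chosen element.
; It also rebuilds the PostProcess settings with a matching scene color tint, so the look updates at construction time.
; The event graph holds no logic.
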(event EventBeginPlay)

(event Collision|EventActorBeginOverlap
  (params (OtherActor :type Actor%20Object%20Reference)))

(event EventTick
  (params (DeltaSeconds :type Float%20%28single-precision%29)))

(fn ConstructionScript
  (bind _returnvalue (Rendering|Material|CreateDynamicMaterialInstance "/Game/Assets/Materials/ToonWater_Master.ToonWater_Master" :!class /Script/Engine.KismetMaterialLibrary))
  (Rendering|Material|SetMaterial (Variables|Default|GetSurface) 0 _returnvalue)
  (Variables|Default|SetSurfaceMatInst _returnvalue)
  (switch Utilities|FlowControl|Switch|SwitchonEElement (Variables|GamePlay|GetElement)
    (:Element_Fire
      (Rendering|Material|SetTextureParameterValue (Variables|Default|GetSurfaceMatInst) "TexParam" "/Game/Assets/Textures/LavaToonTex.LavaToonTex")
      (Variables|/Script/Engine.PostProcessComponent|SetSettings (Variables|Default|GetPostProcess) (Utilities|Struct|MakePostProcessSettings "(R=1.000000,G=0.073312,B=0.000000,A=1.000000)" "DOFM_Gaussian")))
    (:Element_Water
      (Rendering|Material|SetTextureParameterValue (Variables|Default|GetSurfaceMatInst) "TexParam" "/Game/Assets/Textures/WaterToonTex.WaterToonTex")
      (Variables|/Script/Engine.PostProcessComponent|SetSettings (Variables|Default|GetPostProcess) (Utilities|Struct|MakePostProcessSettings "(R=0.000000,G=0.327850,B=0.395833,A=1.000000)" "DOFM_Gaussian")))
    (:Element_Poison
      (Rendering|Material|SetTextureParameterValue (Variables|Default|GetSurfaceMatInst) "TexParam" "/Game/Assets/Textures/PoisonToonTex.PoisonToonTex")
      (Variables|/Script/Engine.PostProcessComponent|SetSettings (Variables|Default|GetPostProcess) (Utilities|Struct|MakePostProcessSettings "(R=0.009467,G=0.203125,B=0.021937,A=1.000000)" "DOFM_Gaussian")))))