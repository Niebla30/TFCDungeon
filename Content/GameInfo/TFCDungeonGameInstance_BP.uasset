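; Game instance for TFCDungeon that handles multiplayer session hosting and joining.
; SessionHost and JoinHost each call DestroySession, then create or join a session without acting on the destroy result.
; A successful host sets ImHost and opens BaseLevel as a listen server, while a successful join clears the flag.
; Successes and create or join failures are reported with on-screen prints.
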(event Custom|SessionHost
  (params (PublicConnections :type Integer) (bUseLAN :type Boolean))
  (bind _returnvalue (Game|GetPlayerController 0))
  ;[1 1 1] Session Host Create Event
  (|DestroySession _returnvalue
    (:then
      _)
    (:OnSuccess
      _)
    (:OnFailure
      _))
  (|Session _returnvalue PublicConnections bUseLAN
    (:OnSuccess
      (Variables|Default|SetImHost true)
      (Development|PrintString "Session created")
      (Game|OpenLevel(byName) "BaseLevel" false "listen"))
    (:OnFailure
      (Development|PrintString "Error creating Session"))))

(event Custom|JoinHost
  (params (SearchResult :type Blueprint%20Session%20Result%20Structure%20%28by%20ref%29))
  (bind _returnvalue (Game|GetPlayerController 0))
  ;[1 1 1] Join to Host Event
  (|DestroySession _returnvalue
    (:then
      _)
    (:OnSuccess
      _)
    (:OnFailure
      _))
  (|JoinSession _returnvalue SearchResult
    (:OnSuccess
      (Variables|Default|SetImHost false)
      (Development|PrintString "Joined to Host"))
    (:OnFailure
      (Development|PrintString "Error joining Session"))))