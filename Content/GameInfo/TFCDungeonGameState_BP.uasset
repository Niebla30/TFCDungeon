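; Dungeon game state Blueprint that listens for state changes on the level's end points.
; On BeginPlay it finds all EndPoint_BP actors and binds a separate handler to the EndPointBehaviour change event of the first two, by array index.
; Both handlers forward the owner character and new state to EndPointChangeStateResponse, whose logic is not defined in this graph.
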(event Custom|EndPointChanged_1
  (params (OwnerCharacter :type ECharacter%20Enum :default "Char_FireBoy") (EndPointState :type EEndPointState%20Enum :default "State_Busy"))
  (Class|TFCDungeonGameState|EndPointChangeStateResponse OwnerCharacter EndPointState))

(event Custom|EndPointChanged_0
  (params (OwnerCharacter :type ECharacter%20Enum :default "Char_FireBoy") (EndPointState :type EEndPointState%20Enum :default "State_Busy"))
  (Class|TFCDungeonGameState|EndPointChangeStateResponse OwnerCharacter EndPointState))

(event EventBeginPlay
  (bind _outactors (Actor|GetAllActorsOfClass "/Game/Assets/Dynamic/EndPoint/EndPoint_BP.EndPoint_BP_C"))
  (Utilities|FlowControl|Sequence
    (:then_0
      (EventDispatchers|BindEventtoOnEndPointChangeState (Variables|/Game/Assets/Dynamic/EndPoint/EndPoint_BP.EndPoint_BP_C|GetEndPointBehaviour (Utilities|Array|Get(acopy) _outactors)) (delegate Custom|EndPointChanged_0)))
    (:then_1
      (EventDispatchers|BindEventtoOnEndPointChangeState (Variables|/Game/Assets/Dynamic/EndPoint/EndPoint_BP.EndPoint_BP_C|GetEndPointBehaviour (Utilities|Array|Get(acopy) _outactors 1)) (delegate Custom|EndPointChanged_1)))))

(event EventTick
  (params (DeltaSeconds :type Float%20%28single-precision%29)))

(fn ConstructionScript)